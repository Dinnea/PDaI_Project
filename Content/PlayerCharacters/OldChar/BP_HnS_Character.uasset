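; BP_HnS_Character is a player character Blueprint with an unfinished look-at feature.
; Its LookAt event takes a target X and Y, computes a rotation from the actor's location, stores it in TargetRotation and prints it.
; A disconnected chain would turn the actor toward that rotation with constant-speed RInterpToConstant, but Tick is empty, so the actor never rotates here.
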(event `Event LookAt`
  (params (`Target X` :type "Float (double-precision)") (`Target Y` :type "Float (double-precision)"))
  (bind (_returnvalue_x _returnvalue_y) (`KismetMathLibrary.BreakVector` (`self.K2_GetActorLocation`)))
  (bind _output_get (set `self.TargetRotation` (`KismetMathLibrary.FindLookAtRotation` (`KismetMathLibrary.MakeVector` _returnvalue_x _returnvalue_y) (`KismetMathLibrary.MakeVector` `Target X` `Target Y`))))
  (`KismetSystemLibrary.PrintString` (`KismetStringLibrary.Conv_RotatorToString` _output_get)))

(event `self.ReceiveBeginPlay`)

(event `self.ReceiveTick`
  (params (DeltaSeconds :type "Float (single-precision)")))

(fn `UserConstructionScript`)